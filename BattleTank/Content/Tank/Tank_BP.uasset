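; Player-drivable tank pawn with aiming, firing, switchable first and third-person cameras and a health bar widget.
; BeginPlay hands the tracks to the movement component, turret and barrel to the aiming component, and itself to the health bar UI.
; Input rotates the camera gimbal and spring arm, triggers fire, and drives either fly-by-wire movement or individual track throttles.
; The construction script sets track meshes and physical materials to work around engine bugs.
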(event EventBeginPlay
  ;[1 1 1] Initalize Tank Movement
  (Class|TankMovementComponent|Initialize (Variables|Default|GetTankMovement) (Variables|Default|GetTankTrackLeft) (Variables|Default|GetTankTrackRight))
  ;[1 1 1] Set turret and barrel references to the Aiming Component
  (Class|TankAimingComponent|SetTurretReference (Variables|Default|GetTankAiming) (Variables|Default|GetTankTurret))
  (Class|TankAimingComponent|SetBarrelReference (Variables|Default|GetTankAiming) (Variables|Default|GetTankBarrel))
  ;[1 1 1] Cast the "Health As A Percent" C++ functionality to the HeatlhBarUI
  (CallFunction|InitalizeHealthBarWidgetUI))

(event Input|ActionEvents|InputActionFire
  (params (Key :type Key%20Structure :default "None"))
  ;[1 1 1] Keyboard/Gamepad Input Binding
  (:Pressed
    (Class|TankAimingComponent|Fire (Variables|Default|GetTankAiming))))

(event Input|ActionEvents|InputActionSwapCamera
  (params (Key :type Key%20Structure :default "None"))
  ;[1 1 1] Swap Camera Controls
  (:Pressed
    (Components|Activation|ToggleActive (Variables|Default|Get1stPersonCamera))
    (Components|Activation|ToggleActive (Variables|Default|Get3rdPersonCamera))))

(event Input|AxisEvents|InputAxisAimAzimuth
  (params (AxisValue :type Float%20%28single-precision%29))
  ;[1 1 1] Camera Input Binding
  (Transformation|AddLocalRotation (Variables|Default|GetAzimuthGimbal) (Math|Rotator|MakeRotator 0.0 0.0 AxisValue) false false))

(event Input|AxisEvents|InputAxisAimElevation
  (params (AxisValue :type Float%20%28single-precision%29))
  ;[1 1 1] Camera Input Binding
  (Transformation|AddLocalRotation (Variables|Default|GetSpringArm) (Math|Rotator|MakeRotator 0.0 AxisValue 0.0) false false))

(event Input|AxisEvents|InputAxisLeftTrackThrottle
  (params (AxisValue :type Float%20%28single-precision%29))
  ;[1 1 1] Keyboard/Gamepad Input Binding
  (Class|TankTrack|SetThrottle (Variables|Default|GetTankTrackLeft) AxisValue))

(event Input|AxisEvents|InputAxisRightTrackThrottle
  (params (AxisValue :type Float%20%28single-precision%29))
  ;[1 1 1] Keyboard/Gamepad Input Binding
  (Class|TankTrack|SetThrottle (Variables|Default|GetTankTrackRight) AxisValue))

(event Input|AxisEvents|InputAxisMoveForward
  (params (AxisValue :type Float%20%28single-precision%29))
  ;[1 1 1] Fly-by-wire control system (using analogue left thumb stick)
  (Class|TankMovementComponent|IntendMoveForward (Variables|Default|GetTankMovement) AxisValue))

(event Input|AxisEvents|InputAxisTurnRight
  (params (AxisValue :type Float%20%28single-precision%29))
  ;[1 1 1] Fly-by-wire control system (using analogue left thumb stick)
  (Class|TankMovementComponent|IntendTurnRight (Variables|Default|GetTankMovement) AxisValue))

(fn ConstructionScript
  ;[1 1 1] Set track mesh using BP (due to bug)
  (Components|StaticMesh|SetStaticMesh (Variables|Default|GetTankTrackLeft) "/Game/Tank/TankModel/tank_fbx_Track.tank_fbx_Track")
  (Components|StaticMesh|SetStaticMesh (Variables|Default|GetTankTrackRight) "/Game/Tank/TankModel/tank_fbx_Track.tank_fbx_Track")
  ;[1 1 1] Set track's phys material (also due to hot reload bug)
  (Class|PrimitiveComponent|SetPhysMaterialOverride (Variables|Default|GetTankTrackLeft) "/Game/Tank/PhysMat_Track.PhysMat_Track")
  (Class|PrimitiveComponent|SetPhysMaterialOverride (Variables|Default|GetTankTrackRight) "/Game/Tank/PhysMat_Track.PhysMat_Track"))

(fn InitalizeHealthBarWidgetUI
  (bind _ashealth_bar_ui (Utilities|Casting|CastToHealthBarUI (UserInterface|GetUserWidgetObject (Variables|Default|GetHealthBar))))
  (Variables|/Game/_UI/HealthBarUI.HealthBarUI_C|SetTankRef _ashealth_bar_ui self))